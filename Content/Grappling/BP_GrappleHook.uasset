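; BP_GrappleHook is a grapple hook projectile that flies in a straight line toward its CurrentTarget and stops there.
; BeginPlay caches start and target locations, then launches ProjectileMovement along that direction at ProjectileSpeed.
; Tick compares squared distances from the start against the target's current location, then snaps to the cached end point and zeroes velocity on arrival or overshoot.
; DistanceToTarget returns the remaining distance to that cached end point.
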(event `self.ReceiveBeginPlay`
  (set `self.StartLoc` (`self.K2_GetActorLocation`))
  (set `self.EndLoc` (`self.K2_GetActorLocation` (`self.CurrentTarget`)))
  (set `self.Direction` (`KismetMathLibrary.Normal` (- (`self.EndLoc`) (`self.StartLoc`))))
  (set `MovementComponent.Velocity` (* (`self.Direction`) (`self.ProjectileSpeed`)) (`self.ProjectileMovement`)))

(event `self.ReceiveTick`
  (params (DeltaSeconds :type "Float (single-precision)"))
  (if (>= (`KismetMathLibrary.Vector_DistanceSquared` (`self.K2_GetActorLocation`) (`self.StartLoc`)) (`KismetMathLibrary.Vector_DistanceSquared` (`self.K2_GetActorLocation` (`self.CurrentTarget`)) (`self.StartLoc`)))
    (`self.K2_SetActorLocation` (+ (`self.StartLoc`) (* (`self.Direction`) (`KismetMathLibrary.Vector_Distance` (`self.StartLoc`) (`self.EndLoc`)))))
    (set `MovementComponent.Velocity` (0.0 0.0 0.0) (`self.ProjectileMovement`))))

(fn `DistanceToTarget`
  (returns (ReturnValue :type "Float (double-precision)"))
  (return (`KismetMathLibrary.Vector_Distance` (`self.EndLoc`) (`self.K2_GetActorLocation`))))

(fn `UserConstructionScript`)